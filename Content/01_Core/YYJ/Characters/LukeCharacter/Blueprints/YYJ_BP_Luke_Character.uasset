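; Luke's character Blueprint, implementing an aim-and-throw grenade skill on the skill input action.
; While the input triggers, it sets an aiming flag and predicts the projectile path from GrenadeRef, shown only through debug drawing as the path-point loop is empty.
; On release it plays the throw montage, whose notify spawns a grenade and sets its physics velocity along the actor-to-GrenadeRef direction at GrenadeSpeed.
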(event `EnhancedInput|/Game/01_Core/YYJ/Input/InputAction/YYJ_IA_Skill`
  (params (ActionValue :type Boolean) (ElapsedSeconds :type "Float (double-precision)") (TriggeredSeconds :type "Float (double-precision)") (InputAction :type "InputAction Object Reference" :default "/Game/01_Core/YYJ/Input/InputAction/YYJ_IA_Skill.YYJ_IA_Skill"))
  (bind _returnvalue (`SceneComponent.K2_GetComponentLocation` (`self.GrenadeRef`)))
  (:`Triggered`
    (`|PlayMontage` (`self.Mesh`)
      (:`then`
        (set `self.bIsGrenadeAim` true)
        (bind _predictresult (`GameplayStatics.Blueprint_PredictProjectilePath_Advanced` (make `PredictProjectilePathParams` _returnvalue (* (`KismetMathLibrary.GetDirectionUnitVector` (`self.K2_GetActorLocation`) _returnvalue) (`self.GrenadeSpeed`)) true 16.0 3.0 true "ECC_WorldStatic" _ (`|MakeArray` self :!type "Actor Object Reference") 20.0 0.0 "ForOneFrame")))
        (for _ (break `PredictProjectilePathResult` _predictresult)
          _))))
  (:`Completed`
    (`|PlayMontage` (`self.Mesh`) "/Game/01_Core/YYJ/Characters/LukeCharacter/Animations/Montage/YYJ_AM_GrenadeThrow.YYJ_AM_GrenadeThrow"
      (:`then`
        (set `self.bIsGrenadeAim` false))
      (:`OnNotifyBegin`
        (bind _returnvalue_2 (`|SpawnActorFromClass` "/Game/01_Core/YYJ/Characters/LukeCharacter/Blueprints/YYJ_BP_Grenade.YYJ_BP_Grenade_C" (`KismetMathLibrary.MakeTransform` (`SceneComponent.K2_GetComponentLocation` (`self.GrenadeRef`)) (`self.K2_GetActorRotation`)) "Undefined" "MultiplyWithRoot" null null))
        (`PrimitiveComponent.SetPhysicsLinearVelocity` (`/Game/01_Core/YYJ/Characters/LukeCharacter/Blueprints/YYJ_BP_Grenade.Sphere` _returnvalue_2) (* (`KismetMathLibrary.GetDirectionUnitVector` (`self.K2_GetActorLocation`) (`self.K2_GetActorLocation` _returnvalue_2)) (`self.GrenadeSpeed`)) false "None")))))

(fn `UserConstructionScript`
  (`parent.UserConstructionScript`))
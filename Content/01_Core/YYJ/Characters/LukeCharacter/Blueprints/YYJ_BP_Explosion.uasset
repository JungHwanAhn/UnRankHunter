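; Explosion actor that damages and pushes whatever is around it shortly after it spawns.
; On BeginPlay, after a brief delay, it applies full radial damage around a point raised above its root, ignoring itself and using the Camera channel to block damage.
; It then fires its RadialForce impulse and draws a temporary debug sphere showing the damage radius.
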(event `self.ReceiveBeginPlay`
  (bind _returnvalue (+ (`SceneComponent.K2_GetComponentLocation` (`self.DefaultSceneRoot`)) (0.0 0.0 200.0)))
  (`KismetSystemLibrary.Delay` 0.1)
  (`GameplayStatics.ApplyRadialDamage` 200.0 _returnvalue 800.0 "/Script/Engine.DamageType" (`|MakeArray` self :!type "Actor Object Reference") self null true "ECC_Camera")
  (`RadialForceComponent.FireImpulse` (`self.RadialForce`))
  (`KismetSystemLibrary.DrawDebugSphere` _returnvalue 800.0 12 (struct :`R` 0.612976 :`G` 1.0 :`B` 0.405753 :`A` 1.0) 1.0))

(fn `UserConstructionScript`)
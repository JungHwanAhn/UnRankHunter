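; Grenade actor that detonates on a fixed fuse after spawning, with bounce and explosion audio.
; BeginPlay waits out the delay, spawns a separate explosion actor at the mesh, plays the explosion cue, hides the mesh and shortly destroys itself.
; Sphere hits play an attenuated bounce sound, throttled by a flag that resets after a brief delay.
; An explosion particle spawn is left unconnected.
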(event `self.ReceiveBeginPlay`
  (`KismetSystemLibrary.Delay` 2.5)
  (`/Engine/EditorBlueprintResources/StandardMacros.IsValid` "YYJ_BP_Grenade"
    (:`Is Valid`
      (`|SpawnActorFromClass` "/Game/01_Core/YYJ/Characters/LukeCharacter/Blueprints/YYJ_BP_Explosion.YYJ_BP_Explosion_C" (`KismetMathLibrary.MakeTransform` (`SceneComponent.K2_GetComponentLocation` (`self.SM_Grenade`))) "Undefined" "MultiplyWithRoot" null null)
      (`GameplayStatics.PlaySoundAtLocation` "/Game/StarterContent/Audio/Explosion_Cue.Explosion_Cue" (`SceneComponent.K2_GetComponentLocation` (`self.SM_Grenade`)) (struct) 1.0 1.0 0.0 null null null null)
      (`SceneComponent.SetHiddenInGame` (`self.SM_Grenade`) true false)
      (`KismetSystemLibrary.Delay` 0.2)
      (`self.K2_DestroyActor`))))

(event `self.Sphere.OnComponentHit`
  (params (HitComponent :type "PrimitiveComponent Object Reference") (OtherActor :type "Actor Object Reference") (OtherComp :type "PrimitiveComponent Object Reference") (NormalImpulse :type "Vector Structure") (Hit :type "HitResult Structure (by ref)"))
  (if (not (`self.CanPlaySound`))
    (set `self.CanPlaySound` true)
    (`GameplayStatics.PlaySoundAtLocation` "/Game/02_Asset/MilitaryWeapDark/Sound/GrenadeLauncher/GrenadeLauncher_Bounce_Cue.GrenadeLauncher_Bounce_Cue" (`SceneComponent.K2_GetComponentLocation` (`self.Sphere`)) (struct) 0.5 1.0 0.0 "/Game/02_Asset/Sound/SA_Character.SA_Character" null null null)
    (`KismetSystemLibrary.Delay` 0.2)
    (set `self.CanPlaySound` false)))

(fn `UserConstructionScript`)
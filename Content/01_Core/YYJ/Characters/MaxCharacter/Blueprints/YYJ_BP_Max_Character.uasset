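; Max player character Blueprint that adds a Roar skill on the Q input.
; Roar cancels weapon actions, disables input and plays a montage with aura overlay and particle effects, guarded by IsRoar until it ends.
; Montage notify begin and end both trigger RoarDamage, which applies radial damage, fires a RadialForce impulse and spawns a shockwave.
; While roaring, incoming damage is cut to a tenth before reaching the parent handler.
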(event `EnhancedInput|/Game/01_Core/YYJ/Input/InputAction/YYJ_IA_Skill_Q`
  (params (ActionValue :type Boolean) (ElapsedSeconds :type "Float (double-precision)") (TriggeredSeconds :type "Float (double-precision)") (InputAction :type "InputAction Object Reference" :default "/Game/01_Core/YYJ/Input/InputAction/YYJ_IA_Skill_Q.YYJ_IA_Skill_Q"))
  (:`Started`
    (`WeaponInterface.CancelWeaponAction` (`self.KYG_AC_WeaponManager_Player`) "All")
    (if (not (`self.bIsRoar`))
      (`|ExecutionSequence`
        (:`then_0`
          (`self.DisableInput` null)
          (set `self.bIsRoar` true)
          (`|PlayMontage` (`self.Mesh`) "/Game/01_Core/YYJ/Characters/MaxCharacter/Animations/Montage/YYJ_AM_Roar.YYJ_AM_Roar"
            (:`then`
              (bind _returnvalue (`GameplayStatics.SpawnEmitterAttached` "/Game/02_Asset/InfinityBladeEffects/Effects/FX_Skill_RockBurst/P_Health_Absorb_01.P_Health_Absorb_01" (`self.Mesh`) "None" (+ (`self.K2_GetActorLocation`) (0.0 -10.0 40.0)) (struct) (2.0 2.0 2.0) "KeepWorldPosition" true "AutoRelease"))
              (`KismetSystemLibrary.Delay` 0.5)
              (`ActorComponent.SetActive` _returnvalue false false)
              (`KismetSystemLibrary.Delay` 2.63)
              (`self.StopAnimMontage` "/Game/01_Core/YYJ/Characters/MaxCharacter/Animations/Montage/YYJ_AM_Roar.YYJ_AM_Roar")
              (set `self.bIsRoar` false)
              (`self.EnableInput` null)
              (`MeshComponent.SetOverlayMaterial` (`self.Mesh`) null))
            (:`OnNotifyBegin`
              (`self.RoarDamage` :!label _label))
            (:`OnNotifyEnd`
              (goto _label))))
        (:`then_1`
          (`MeshComponent.SetOverlayMaterial` (`self.Mesh`) "/Game/01_Core/YYJ/Characters/MaxCharacter/Materials/YYJ_MI_Aura.YYJ_MI_Aura")
          (`ActorComponent.SetActive` (`self.FocusEffect`) true false))
        (:`then_2`
          (`KismetSystemLibrary.Delay` 0.5)
          (`ActorComponent.SetActive` (`self.FocusEffect`) false false))))))

(event `RoarDamage`
  (`GameplayStatics.ApplyRadialDamage` 100.0 (+ (`self.K2_GetActorLocation`) (0.0 0.0 200.0)) 500.0 "/Script/Engine.DamageType" (`|MakeArray` self :!type "Actor Object Reference") self null true "ECC_Camera")
  (`KismetSystemLibrary.Delay` 0.1)
  (`RadialForceComponent.FireImpulse` (`self.RadialForce`))
  (bind _returnvalue (`NiagaraFunctionLibrary.SpawnSystemAttached` "/Game/02_Asset/MagicSpells/Earth/FX/NS_PulseQuake.NS_PulseQuake" (`self.Mesh`) "None" (- (`self.K2_GetActorLocation`) (0.0 0.0 85.0)) (struct) "KeepWorldPosition" true true "AutoRelease"))
  (`KismetSystemLibrary.Delay` 2.0)
  (`ActorComponent.SetActive` _returnvalue false false))

(event `self.ReceiveAnyDamage`
  (params (Damage :type "Float (single-precision)") (DamageType :type "DamageType Object Reference") (InstigatedBy :type "Controller Object Reference") (DamageCauser :type "Actor Object Reference"))
  (if (`self.bIsRoar`)
    (`parent.ReceiveAnyDamage` (* Damage 0.1) null null null)
    (else
      (`parent.ReceiveAnyDamage` Damage null null null))))

(fn `UserConstructionScript`
  (`parent.UserConstructionScript`))
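; Seol player character Blueprint with a timed Ghost skill that grants speed, invincibility and chain lightning attacks.
; The skill input starts Ghost, which ignores several capsule collision channels and shows a dash effect, then restores everything after a delay.
; While ghosted, enemies entering LightningRange take damage and spawn a Niagara beam, whose endpoints Tick updates for the latest spawn.
; MoveToNearestEnemy holds only disconnected nearest-target search logic.
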(event `self.ReceiveBeginPlay`
  ;[0 0 0] Begin Play
  (`parent.ReceiveBeginPlay`))

(event `self.LightningRange.OnComponentBeginOverlap`
  (params (OverlappedComponent :type "PrimitiveComponent Object Reference") (OtherActor :type "Actor Object Reference") (OtherComp :type "PrimitiveComponent Object Reference") (OtherBodyIndex :type Integer) (bFromSweep :type Boolean) (SweepResult :type "HitResult Structure (by ref)"))
  ;[0 0 0] Chain Lightning
  (if (`self.bIsGhost`)
    (set `self.bIsLightning` true)
    (`/Engine/EditorBlueprintResources/StandardMacros.IsValid` OtherActor
      (:`Is Valid`
        (if (`self.ActorHasTag` OtherActor "Enemy")
          (bind _returnvalue (`NiagaraFunctionLibrary.SpawnSystemAttached` "/Game/01_Core/YYJ/Characters/SeolCharacter/VFX/YYJ_NS_ChainLightning.YYJ_NS_ChainLightning" (`self.Mesh`) "None" (`self.K2_GetActorLocation`) (struct) "KeepWorldPosition" false true "AutoRelease"))
          (set `self.ChainLight_Ref` _returnvalue)
          (`GameplayStatics.ApplyDamage` OtherActor 20.0 null self))))))

(event `EnhancedInput|/Game/01_Core/YYJ/Input/InputAction/YYJ_IA_Skill`
  (params (ActionValue :type Boolean) (ElapsedSeconds :type "Float (double-precision)") (TriggeredSeconds :type "Float (double-precision)") (InputAction :type "InputAction Object Reference" :default "/Game/01_Core/YYJ/Input/InputAction/YYJ_IA_Skill.YYJ_IA_Skill"))
  ;[0 0 0] Skill
  (:`Started`
    (if (not (`self.bIsGhost`))
      (`self.Ghost`))))

(event `self.ReceiveTick`
  (params (DeltaSeconds :type "Float (single-precision)"))
  (bind _chainlight_ref (`self.ChainLight_Ref`))
  (bind _returnvalue_location (`KismetMathLibrary.BreakTransform` (`SceneComponent.GetSocketTransform` (`self.Mesh`) "spine_01Socket_Skill" "RTS_World")))
  ;[0 0 0] Chain Lightning Location
  (`/Engine/EditorBlueprintResources/StandardMacros.IsValid` (`self.ChainLight_Ref`)
    (:`Is Valid`
      (`FXSystemComponent.SetVectorParameter` _chainlight_ref "BeamStartPoint" _returnvalue_location)
      (`FXSystemComponent.SetVectorParameter` _chainlight_ref "BeamEndPoint" (`self.K2_GetActorLocation` (stale `self.LightningRange.OnComponentBeginOverlap` OtherActor))))))

(event `Ghost`
  (bind _capsulecomponent (`self.CapsuleComponent`))
  (bind _capsulecomponent_2 (`self.CapsuleComponent`))
  ;[0 0 0] Ghost
  (set `self.bIsGhost` true)
  (set `self.bIsInvincible` true)
  (set `CharacterMovementComponent.MaxWalkSpeed` 1500.0 (`self.CharacterMovement`))
  (`PrimitiveComponent.SetCollisionResponseToChannel` _capsulecomponent_2 "ECC_PhysicsBody" "ECR_Ignore")
  (`PrimitiveComponent.SetCollisionResponseToChannel` _capsulecomponent_2 "ECC_Pawn" "ECR_Ignore")
  (`PrimitiveComponent.SetCollisionResponseToChannel` _capsulecomponent_2 "ECC_GameTraceChannel1" "ECR_Ignore")
  (`PrimitiveComponent.SetCollisionResponseToChannel` _capsulecomponent_2 "ECC_WorldDynamic" "ECR_Ignore")
  (`ActorComponent.SetActive` (`self.NS_Dash_07`) true false)
  (`KismetSystemLibrary.Delay` 5.0)
  (`ActorComponent.SetActive` (`self.NS_Dash_07`) false false)
  (set `self.bIsGhost` false)
  (set `self.bIsInvincible` false)
  (set `CharacterMovementComponent.MaxWalkSpeed` 700.0 (`self.CharacterMovement`))
  (`PrimitiveComponent.SetCollisionResponseToChannel` _capsulecomponent "ECC_PhysicsBody" "ECR_Block")
  (`PrimitiveComponent.SetCollisionResponseToChannel` _capsulecomponent "ECC_Pawn" "ECR_Block")
  (`PrimitiveComponent.SetCollisionResponseToChannel` _capsulecomponent "ECC_GameTraceChannel1" "ECR_Block")
  (`PrimitiveComponent.SetCollisionResponseToChannel` _capsulecomponent "ECC_WorldDynamic" "ECR_Block"))

(event `self.ReceiveAnyDamage`
  (params (Damage :type "Float (single-precision)") (DamageType :type "DamageType Object Reference") (InstigatedBy :type "Controller Object Reference") (DamageCauser :type "Actor Object Reference"))
  ;[0 0 0] Damage
  (if (not (`self.bIsInvincible`))
    (`parent.ReceiveAnyDamage` Damage null null null)))

(fn `MoveToNearestEnemy`)

(fn `UserConstructionScript`
  (`parent.UserConstructionScript`))
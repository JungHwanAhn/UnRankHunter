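; Skill actor for its owning YYJ base character that provides a five-second Ghost dash state with chain lightning.
; The Ghost event sets an invincibility flag, raises walk speed, ignores several capsule collision channels and activates dash Niagara, then reverts.
; During Ghost, overlapping an Enemy-tagged actor with LightningRange spawns a lightning beam and applies damage.
; Tick updates the latest beam between the owner's spine socket and the overlapped actor; the E input does nothing.
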(event `self.ReceiveBeginPlay`
  (bind _asyyj_bp_base_character (cast `/Game/01_Core/YYJ/Characters/BaseCharacter/Blueprints/YYJ_BP_Base_Character` (`self.GetOwner`)))
  (`/Engine/EditorBlueprintResources/StandardMacros.IsValid` _asyyj_bp_base_character
    (:`Is Valid`
      (set `self.As YYJ BP Base Character` _asyyj_bp_base_character))))

(event `EnhancedInput|/Game/01_Core/YYJ/Input/InputAction/YYJ_IA_Skill_E`
  (params (ActionValue :type Boolean) (ElapsedSeconds :type "Float (double-precision)") (TriggeredSeconds :type "Float (double-precision)") (InputAction :type "InputAction Object Reference" :default "/Game/01_Core/YYJ/Input/InputAction/YYJ_IA_Skill_E.YYJ_IA_Skill_E"))
  (:`Started`
    (if (`self.bIsGhost`)
      _)))

(event `self.LightningRange.OnComponentBeginOverlap`
  (params (OverlappedComponent :type "PrimitiveComponent Object Reference") (OtherActor :type "Actor Object Reference") (OtherComp :type "PrimitiveComponent Object Reference") (OtherBodyIndex :type Integer) (bFromSweep :type Boolean) (SweepResult :type "HitResult Structure (by ref)"))
  (if (`self.bIsGhost`)
    (set `self.bIsLightning` true)
    (`/Engine/EditorBlueprintResources/StandardMacros.IsValid` OtherActor
      (:`Is Valid`
        (if (`self.ActorHasTag` OtherActor "Enemy")
          (bind _returnvalue (`NiagaraFunctionLibrary.SpawnSystemAttached` "/Game/01_Core/YYJ/Characters/SeolCharacter/VFX/YYJ_NS_ChainLightning.YYJ_NS_ChainLightning" null "None" (0.0 0.0 0.0) (struct) "KeepWorldPosition" false true "AutoRelease"))
          (set `self.ChainLightningRef` _returnvalue)
          (`GameplayStatics.ApplyDamage` null 20.0 null self))))))

(event `self.ReceiveTick`
  (params (DeltaSeconds :type "Float (single-precision)"))
  (bind _chainlightningref (`self.ChainLightningRef`))
  (bind _returnvalue_location (`KismetMathLibrary.BreakTransform` (`SceneComponent.GetSocketTransform` (`Character.Mesh` (`self.As YYJ BP Base Character`)) "spine_01Socket_Skill" "RTS_World")))
  (`/Engine/EditorBlueprintResources/StandardMacros.IsValid` (`self.ChainLightningRef`)
    (:`Is Valid`
      (`FXSystemComponent.SetVectorParameter` _chainlightningref "BeamStartPoint" _returnvalue_location)
      (`FXSystemComponent.SetVectorParameter` _chainlightningref "BeamEndPoint" (`self.K2_GetActorLocation` (stale `self.LightningRange.OnComponentBeginOverlap` OtherActor))))))

(event `Ghost`
  (bind _capsulecomponent (`Character.CapsuleComponent` (`self.As YYJ BP Base Character`)))
  (bind _capsulecomponent_2 (`Character.CapsuleComponent` (`self.As YYJ BP Base Character`)))
  (set `self.bIsGhost` true)
  (set `self.bIsInvincible` true)
  (set `CharacterMovementComponent.MaxWalkSpeed` 1500.0 (`Character.CharacterMovement` (`self.As YYJ BP Base Character`)))
  (`PrimitiveComponent.SetCollisionResponseToChannel` _capsulecomponent_2 "ECC_PhysicsBody" "ECR_Ignore")
  (`PrimitiveComponent.SetCollisionResponseToChannel` _capsulecomponent_2 "ECC_Pawn" "ECR_Ignore")
  (`PrimitiveComponent.SetCollisionResponseToChannel` _capsulecomponent_2 "ECC_GameTraceChannel1" "ECR_Ignore")
  (`PrimitiveComponent.SetCollisionResponseToChannel` _capsulecomponent_2 "ECC_WorldDynamic" "ECR_Ignore")
  (`ActorComponent.SetActive` (`self.NS_Dash_07`) true false)
  (`KismetSystemLibrary.Delay` 5.0)
  (`ActorComponent.SetActive` (`self.NS_Dash_07`) false false)
  (set `self.bIsGhost` false)
  (set `self.bIsInvincible` false)
  (set `CharacterMovementComponent.MaxWalkSpeed` 700.0 (`Character.CharacterMovement` (`self.As YYJ BP Base Character`)))
  (`PrimitiveComponent.SetCollisionResponseToChannel` _capsulecomponent "ECC_PhysicsBody" "ECR_Block")
  (`PrimitiveComponent.SetCollisionResponseToChannel` _capsulecomponent "ECC_Pawn" "ECR_Block")
  (`PrimitiveComponent.SetCollisionResponseToChannel` _capsulecomponent "ECC_GameTraceChannel1" "ECR_Block")
  (`PrimitiveComponent.SetCollisionResponseToChannel` _capsulecomponent "ECC_WorldDynamic" "ECR_Block"))

(fn `UserConstructionScript`)
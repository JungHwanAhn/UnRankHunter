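; Actor component that tracks a character's health and shield stats.
; Both current values start at their maximums on BeginPlay.
; Increase functions clamp to the maximum, while decrease functions subtract without a floor and return true once the value reaches zero or below.
; Health and shield are handled independently, with no damage spillover between them.
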(event `self.ReceiveBeginPlay`
  (set `self.CurrentHealth` (`self.MaxHealth`))
  (set `self.CurrentShield` (`self.MaxShield`)))

(fn `Decrease Health`
  (params (Damage :type "Float (double-precision)"))
  (returns (bIsDie :type Boolean))
  (set `self.CurrentHealth` (- (`self.CurrentHealth`) Damage))
  (if (<= (`self.CurrentHealth`) 0.0)
    (return true)
    (else
      (return false))))

(fn `Decrease Shield`
  (params (`Decreased Shield` :type "Float (double-precision)"))
  (returns (bIsShieldNotLeft :type Boolean))
  (set `self.CurrentShield` (- (`self.CurrentShield`) `Decreased Shield`))
  (if (<= (`self.CurrentShield`) 0.0)
    (return true)
    (else
      (return false))))

(fn `Increase Health`
  (params (`Added Health` :type "Float (double-precision)"))
  (set `self.CurrentHealth` (+ (`self.CurrentHealth`) `Added Health`))
  (if (> (`self.CurrentHealth`) (`self.MaxHealth`))
    (set `self.CurrentHealth` (`self.MaxHealth`))))

(fn `Increase Shield`
  (params (`Added Shield` :type "Float (double-precision)"))
  (set `self.CurrentShield` (+ (`self.CurrentShield`) `Added Shield`))
  (if (> (`self.CurrentShield`) (`self.MaxShield`))
    (set `self.CurrentShield` (`self.MaxShield`))))